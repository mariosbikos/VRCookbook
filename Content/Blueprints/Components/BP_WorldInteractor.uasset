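; Scene component that lets its owner hover, drag, use, pick up and drop world objects.
; While enabled, Tick runs a sphere overlap at its location, takes the first result as the hovered object and ends any drag when that changes.
; Interaction events notify objects through messages, with a second gate sending drag updates each tick.
; Pickup asks the object for permission, then snaps it to the component until Drop detaches it.
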(event Custom|Enable
  (Utilities|FlowControl|Gate false) ; enters at Open
)

(event Custom|Disable
  (Utilities|FlowControl|Gate false) ; enters at Close
)

(event Custom|StopDrag
  (if (Variables|Default|GetDragging)
    (Variables|Default|SetDragging false)
    (Class|BPControllerTraceInteractionInterface|OnDragEnd(Message) (Variables|Default|GetHoveredObject) self)
    (Utilities|FlowControl|Gate true) ; enters at Close
  ))

(event Custom|StartDrag
  (Variables|Default|SetDragging true)
  (Class|BPControllerTraceInteractionInterface|OnDragStart(Message) (Variables|Default|GetHoveredObject) self)
  (Utilities|FlowControl|Gate true) ; enters at Open
)

(event Custom|Pickup
  (bind _hoveredobject (Variables|Default|GetHoveredObject))
  (Utilities|IsValid _hoveredobject
    (:Is%20Valid
      (bind _pickup (Class|BPControllerTraceInteractionInterface|CanPickup(Message) _hoveredobject))
      (if _pickup
        (bind _output_get (Variables|Default|SetPickedUpObject (Variables|Default|GetHoveredObject)))
        (Transformation|AttachComponentToComponent _output_get self "None" "SnapToTarget" "SnapToTarget" "KeepWorld" true)
        (Class|BPControllerTraceInteractionInterface|OnPickup(Message) (Variables|Default|GetPickedUpObject) self)))))

(event Custom|Drop
  (Utilities|IsValid (Variables|Default|GetPickedUpObject)
    (:Is%20Valid
      (Transformation|DetachFromActor (Variables|Default|GetPickedUpObject) "KeepWorld" "KeepWorld" "KeepWorld")
      (Class|BPControllerTraceInteractionInterface|OnDrop(Message) (Variables|Default|GetPickedUpObject) self)
      (Variables|Default|SetHoveredObject 0)
      (Variables|Default|SetPickedUpObject 0))))

(event Custom|UseHoveredObject
  ;[1 1 1] For Buttons and things that can be used when player hovers over them
  (Class|BPControllerTraceInteractionInterface|OnUse(Message) (Variables|Default|GetHoveredObject) self))

(event EventTick
  (params (DeltaSeconds :type Float%20%28single-precision%29))
  (Utilities|FlowControl|Gate false
    (:Exit
      (Utilities|FlowControl|Sequence
        (:then_0
          (bind _outactors (Collision|SphereOverlapActors (Transformation|GetWorldLocation) (Variables|Default|GetRadius) (Utilities|Array|MakeArray "ObjectTypeQuery2" "ObjectTypeQuery4") 0 (Utilities|Array|MakeArray (Components|GetOwner))))
          (if (!= (Utilities|Array|Get(acopy) _outactors) (Variables|Default|GetHoveredObject))
            (Class|BPControllerTraceInteractionInterface|OnUnhover(Message) (Variables|Default|GetHoveredObject) self)
            (CallFunction|StopDrag)
            (bind _output_get (Variables|Default|SetHoveredObject (Utilities|Array|Get(acopy) _outactors)))
            (Class|BPControllerTraceInteractionInterface|OnHover(Message) _output_get self)))
        (:then_1
          (Utilities|FlowControl|Gate true
            (:Exit
              (Class|BPControllerTraceInteractionInterface|OnDrag(Message) (Variables|Default|GetHoveredObject) self))))))))