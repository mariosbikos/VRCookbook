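; BP_ControllerInteractionPawn is a VR pawn that maps motion controller input to world interaction for both hands.
; Each hand has its own BPWorldInteractor component that receives that controller's input.
; Grip press and release trigger Pickup and Drop.
; Trigger press uses the hovered object and starts a drag, and trigger release stops the drag.
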(event Input|KeyboardEvents|MotionControllerRightGrip1
  (params (Key :type Key%20Structure))
  (bind _bp_worldinteractor_r (Variables|Default|GetBP_WorldInteractor_R))
  ;[1 1 1] RIGHT CONTROLLER
  (:Pressed
    (Default|Pickup _bp_worldinteractor_r))
  (:Released
    (Default|Drop _bp_worldinteractor_r)))

(event Input|KeyboardEvents|MotionControllerRightTrigger
  (params (Key :type Key%20Structure))
  ;[1 1 1] RIGHT CONTROLLER
  (:Pressed
    (Default|UseHoveredObject (Variables|Default|GetBP_WorldInteractor_R))
    (Default|StartDrag (Variables|Default|GetBP_WorldInteractor_R)))
  (:Released
    (Default|StopDrag (Variables|Default|GetBP_WorldInteractor_R))))

(event Input|KeyboardEvents|MotionControllerLeftGrip1
  (params (Key :type Key%20Structure))
  (bind _bp_worldinteractor_l (Variables|Default|GetBP_WorldInteractor_L))
  ;[1 1 1] LEFT CONTROLLER
  (:Pressed
    (Default|Pickup _bp_worldinteractor_l))
  (:Released
    (Default|Drop _bp_worldinteractor_l)))

(event Input|KeyboardEvents|MotionControllerLeftTrigger
  (params (Key :type Key%20Structure))
  ;[1 1 1] LEFT CONTROLLER
  (:Pressed
    (Default|UseHoveredObject (Variables|Default|GetBP_WorldInteractor_L))
    (Default|StartDrag (Variables|Default|GetBP_WorldInteractor_L)))
  (:Released
    (Default|StopDrag (Variables|Default|GetBP_WorldInteractor_L))))

(fn ConstructionScript)