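; Blueprint interface for objects that a world interactor, by its name a controller trace, can act on.
; It declares hover, unhover, use, pickup, drop and drag start, update and end functions, each receiving the interactor and returning a value.
; A CanPickup query lets implementers report whether they can be picked up.
; The interface holds no logic of its own, so implementing actors supply all behaviour.
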(fn OnHover
  (params (Interactor :type BP%20World%20Interactor%20Object%20Reference))
  (return false))

(fn OnUnhover
  (params (WorldInteractor :type BP%20World%20Interactor%20Object%20Reference))
  (return false))

(fn OnUse
  (params (WorldInteractor :type BP%20World%20Interactor%20Object%20Reference))
  (return false))

(fn OnPickup
  (params (WorldInteractor :type BP%20World%20Interactor%20Object%20Reference))
  (return false))

(fn OnDrop
  (params (WorldInteractor :type BP%20World%20Interactor%20Object%20Reference))
  (return false))

(fn OnDrag
  (params (WorldInteractor :type BP%20World%20Interactor%20Object%20Reference))
  (return false))

(fn OnDragStart
  (params (WorldInteractor :type BP%20World%20Interactor%20Object%20Reference))
  (return false))

(fn OnDragEnd
  (params (WorldInteractor :type BP%20World%20Interactor%20Object%20Reference))
  (return false))

(fn CanPickup
  (return false))