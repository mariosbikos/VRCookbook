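; Menu actor that shows WBP_MenuWidget on a widget component and is operated through trace interaction callbacks.
; On BeginPlay it caches the widget and binds StartButton, whose click only prints "Open Level" as a placeholder.
; TraceMove feeds hits to WidgetInteraction as custom hit results; TraceActivateUp presses and TraceActivateDown releases the left mouse pointer key, inverse to their names.
; The other trace callbacks are stubs, and every trace function returns false.
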(event Custom|StartButton_Clicked
  (Development|PrintString "Open Level"))

(event EventBeginPlay
  (bind _aswbp_menu_widget (Utilities|Casting|CastToWBP_MenuWidget (UserInterface|GetUserWidgetObject (Variables|Default|GetWidget))))
  (bind _output_get (Variables|Default|SetMenuWidget _aswbp_menu_widget))
  (EventDispatchers|BindEventtoOnClicked (Variables|/Game/UMG/WBP_MenuWidget.WBP_MenuWidget_C|GetStartButton _output_get) (delegate Custom|StartButton_Clicked)))

(event Collision|EventActorBeginOverlap
  (params (OtherActor :type Actor%20Object%20Reference)))

(event EventTick
  (params (DeltaSeconds :type Float%20%28single-precision%29)))

(fn ConstructionScript)

(fn TraceActivateDown
  (params (Hit :type Hit%20Result%20Structure%20%28by%20ref%29) (Instigator :type Pawn%20Object%20Reference%20%28by%20ref%29))
  (Class|WidgetInteractionComponent|ReleasePointerKey (Variables|Default|GetWidgetInteraction) "LeftMouseButton")
  (return false))

(fn TraceActivateUp
  (params (Hit :type Hit%20Result%20Structure%20%28by%20ref%29) (Instigator :type Pawn%20Object%20Reference%20%28by%20ref%29))
  (Class|WidgetInteractionComponent|PressPointerKey (Variables|Default|GetWidgetInteraction) "LeftMouseButton")
  (return false))

(fn TraceHitComponent
  (params (Hit :type Hit%20Result%20Structure) (Component :type Primitive%20Component%20Object%20Reference))
  (return false))

(fn TraceHitObject
  (params (Hit :type Hit%20Result%20Structure))
  (return false))

(fn TraceLeaveComponent
  (params (Hit :type Hit%20Result%20Structure) (Component :type Primitive%20Component%20Object%20Reference))
  (return false))

(fn TraceLeaveObject
  (params (Hit :type Hit%20Result%20Structure))
  (return false))

(fn TraceMove
  (params (Hit :type Hit%20Result%20Structure%20%28by%20ref%29))
  (Class|WidgetInteractionComponent|SetCustomHitResult (Variables|Default|GetWidgetInteraction) Hit)
  (return false))